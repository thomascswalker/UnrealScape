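; BP_USPlayerController is a player controller that moves the player's USCharacter by click-to-move on a tile grid.
; On left-click release it clears persistent debug lines and line-traces under the mouse cursor.
; On a hit, it refreshes the character NavigatorComponent's current grid and tile, converts the hit location to a tile, and tells the navigator to navigate to that tile's world position.
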(event `InputAction|LeftClick`
  (params (Key :type "Key Structure"))
  (:`Released`
    (`KismetSystemLibrary.FlushPersistentDebugLines`)
    (bind (_hitresult _returnvalue) (`self.LineTraceUnderMouseCursor`))
    (if _returnvalue
      (bind _asuscharacter (cast `USCharacter` (`GameplayStatics.GetPlayerPawn` 0)))
      (bind _navigatorcomponent (`USCharacter.NavigatorComponent` _asuscharacter))
      (`NavigatorComponent.UpdateCurrentGrid` _navigatorcomponent)
      (`NavigatorComponent.UpdateCurrentTile` _navigatorcomponent)
      (bind _returnvalue_2 (`Grid.GetTileInfoFromLocation` (`NavigatorComponent.CurrentGrid` _navigatorcomponent) (`.Location` (`GameplayStatics.BreakHitResult` _hitresult))))
      (`NavigatorComponent.Navigate` _navigatorcomponent (`.WorldPosition` (break `TileInfo` _returnvalue_2))))))

(fn `UserConstructionScript`)