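; Grid actor Blueprint that builds tile actors at BeginPlay and visualizes paths between the player's selected tiles.
; Each Tick it clears debug lines, reads CurrentTile and TargetTile from USPlayerController, and converts both to tile info for RequestPath.
; Debug boxes mark the target and each path tile, shaded blue to green along the route.
; Tile construction and pathfinding come from functions defined outside this graph.
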(event `self.ReceiveBeginPlay`
  (`self.ConstructTileActors` (0.0 0.0 0.0)))

(event `self.ReceiveTick`
  (params (DeltaSeconds :type "Float (single-precision)"))
  (`KismetSystemLibrary.FlushPersistentDebugLines`)
  (bind _asusplayer_controller (cast `USPlayerController` (`GameplayStatics.GetPlayerController` 0)))
  (bind _currenttile (`USPlayerController.CurrentTile` _asusplayer_controller))
  (`/Engine/EditorBlueprintResources/StandardMacros.IsValid` _currenttile
    (:`Is Valid`
      (bind _targettile (`USPlayerController.TargetTile` _asusplayer_controller))
      (`/Engine/EditorBlueprintResources/StandardMacros.IsValid` _targettile
        (:`Is Valid`
          (bind _returnvalue (`self.GetTileInfoFromTileActor` _currenttile)) ; Start Tile
          (bind _returnvalue_2 (`self.GetTileInfoFromTileActor` _targettile)) ; End Tile
          (`KismetSystemLibrary.DrawDebugBox` (`.WorldPosition` (break `TileInfo` _returnvalue_2)) (25.0 25.0 5.0) (make `LinearColor` 0.0 1.0) (struct) 1.0 5.0) ; End
          (bind _returnvalue_3 (`self.RequestPath` _returnvalue _returnvalue_2))
          (for (_array_element _array_index) _returnvalue_3
            (bind _returnvalue_4 (- (`KismetArrayLibrary.Array_Length` _returnvalue_3) 1))
            (`KismetSystemLibrary.DrawDebugBox` (`.WorldPosition` (break `TileInfo` _array_element)) (25.0 25.0 5.0) (make `LinearColor` 0.0 (/ _array_index _returnvalue_4) (- 1.0 (/ _array_index _returnvalue_4))) (struct) 1.0 5.0)))))))

(fn `UserConstructionScript`)