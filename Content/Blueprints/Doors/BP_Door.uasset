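; Interactable door Blueprint that players can open, close or examine through named interaction options.
; The Interact event switches on the option name, snapping the door component's yaw between closed and open without animation and tracking the IsOpen state.
; Each toggle renames the option between Open and Close, while Examine logs the current state to the chatbox.
; Every branch ends by signalling interaction completion.
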(event `self.Interact`
  (params (Option :type "InteractOption Structure (by ref)"))
  (bind _door (`self.Door`))
  (switch `string` Option_Name
    (:`Open`
      (`SceneComponent.K2_SetRelativeRotation` _door (struct :`Yaw` -90.0) false false) ; Open the door
      (set `self.bIsOpen` true)
      (`self.SetOptionName` "Open" "Close")
      (`self.InteractionComplete` :!label _label))
    (:`Close`
      (`SceneComponent.K2_SetRelativeRotation` :`self` _door) ; Close the door
      (set `self.bIsOpen` false)
      (`self.SetOptionName` "Close" "Open")
      (goto _label))
    (:`Examine`
      (if (`self.bIsOpen`)
        (`/Game/Blueprints/UI/FBP_Chatbox.Log (Chatbox)` "The door is open.")
        (else
          (`/Game/Blueprints/UI/FBP_Chatbox.Log (Chatbox)` "The door is closed.")))
      (`self.InteractionComplete`))))

(fn `UserConstructionScript`)