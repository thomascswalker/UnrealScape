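; BP_TutIslandDoor1 is an interactive Tutorial Island door, usable only once that quest has started.
; Construction fills its InteractiveComponent from the "Door" row of DT_ObjectData.
; Open and Close rotate the mesh a quarter turn and swap option visibility, while Examine reports the state in chat.
; Any interaction during quest step 1 advances it to step 2; before the quest, a chat message points to the guide.
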(event `self.Interact`
  (params (Option :type "InteractOption Structure (by ref)"))
  (bind _staticmeshcomponent (`self.StaticMeshComponent`))
  (bind _staticmeshcomponent_2 (`self.StaticMeshComponent`))
  (bind (_relativerotation_roll _relativerotation_pitch _relativerotation_yaw) (`KismetMathLibrary.BreakRotator` (`SceneComponent.RelativeRotation` _staticmeshcomponent_2)))
  (set `self.OriginalCollision` (`PrimitiveComponent.GetCollisionEnabled` _staticmeshcomponent_2))
  (set `self.OriginalYaw` _relativerotation_yaw)
  (`QuestFunctionLibrary.IsQuestStarted` "TutorialIsland"
    (:`True`
      (switch `string` (`.Name` (break `InteractOption` Option))
        (:`Open`
          (`SceneComponent.K2_AddRelativeRotation` _staticmeshcomponent (struct :`Yaw` -90.0) false false)
          (bind _output_get (set `self.bIsOpen` (not (`self.bIsOpen`)) :!label _label))
          (if _output_get
            (`self.SetOptionVisibility` "Close" true) ; Door is now open
            (`self.SetOptionVisibility` "Open")
            (else
              (`self.SetOptionVisibility` "Close") ; Door is now closed
              (`self.SetOptionVisibility` "Open" true))))
        (:`Close`
          (`SceneComponent.K2_AddRelativeRotation` _staticmeshcomponent (struct :`Yaw` 90.0) false false)
          (goto _label))
        (:`Examine`
          (`GlobalFunctionLibrary.AddChatboxMessage` (`|FormatText` "The door is {State}." (`KismetMathLibrary.SelectString` "open" "closed" (`self.bIsOpen`))))))
      (`PrimitiveComponent.SetCollisionEnabled` (`self.StaticMeshComponent`) (`self.OriginalCollision`))
      (if (== (`QuestFunctionLibrary.GetQuestStep` "TutorialIsland") 1)
        (`QuestFunctionLibrary.SetQuestStep` "TutorialIsland" 2)))
    (:`False`
      (`GlobalFunctionLibrary.AddChatboxMessage` "You need to speak with the guide first."))))

(fn `UserConstructionScript`
  (bind _interactivecomponent (`self.InteractiveComponent`))
  (`parent.UserConstructionScript`)
  (bind _returnvalue (`|GetDataTableRow` "/Game/Blueprints/Objects/DT_ObjectData.DT_ObjectData" "Door")
    (:`then`
      (bind (_interactdistance _name _type _options) (break `EntityData` _returnvalue))
      (set `InteractiveComponent.InteractDistance` _interactdistance _interactivecomponent)
      (set `InteractiveComponent.Name` _name _interactivecomponent)
      (set `InteractiveComponent.Type` _type _interactivecomponent)
      (set `InteractiveComponent.Options` _options _interactivecomponent))))