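; Tutorial Island quest Blueprint that guides the player through early steps with world hints and starter items.
; Update switches on the step to move hints and hand out a fishing net, then a tinderbox and axe, reverting a step if either of the latter fails.
; An inventory item-added binding advances the quest on raw shrimp.
; Quest completion is bound at the first step, and Reward only prints a placeholder string.
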(event `self.Update`
  (params (Step :type Integer))
  (switch `int` Step
    (:`0`
      (`HintFunctionLibrary.CreateHint` null (2350.0 -650.0 1288.0) true)
      (add `self.QuestCompleted` (`|CreateDelegate` :!event `CustomEvent`)))
    (:`1`
      (`HintFunctionLibrary.CreateHint` null (2350.0 -200.000001 1388.0) true))
    (:`2`
      (`HintFunctionLibrary.CreateHint` null (1250.0 150.0 1100.0) true))
    (:`3`
      (`HintFunctionLibrary.CreateHint` null (990.0 260.0 850.0) true)
      (`ItemFunctionLibrary.GivePlayerItemFromId` null 303 ; Small fishing net
        (:`True`
          (bind _returnvalue (`ItemFunctionLibrary.GetInventoryComponent` null))
          (add `InventoryComponent.ItemAdded` _returnvalue (`|CreateDelegate` :!event `OnShrimpAcquired`)))))
    (:`4`
      (`HintFunctionLibrary.CreateHint` null (1250.0 150.0 1100.0) true)
      (remove `InventoryComponent.ItemAdded` _returnvalue (`|CreateDelegate` :!event `OnShrimpAcquired`)))
    (:`5`
      (`HintFunctionLibrary.ClearHints` null)
      (`ItemFunctionLibrary.GivePlayerItemFromId` null 590 ; Tinderbox
        (:`True`
          (`ItemFunctionLibrary.GivePlayerItemFromId` null 1351 ; Bronze Axe
            (:`False`
              _)))
        (:`False`
          _))
      (`QuestFunctionLibrary.SetQuestStep` null "TutorialIsland" 4))))

(event `OnShrimpAcquired`
  (params (ItemDef :type "ItemDef Structure") (Count :type Integer))
  (if (== (`.Id` (break `ItemDef` ItemDef)) 317)
    (bind _output_get (set `self.CurrentStep` 4))
    (`self.Update` _output_get)))

(event `self.Reward`
  (`KismetSystemLibrary.PrintString` null "reward"))

(event `CustomEvent` :!signature `self.QuestCompleted`
  (params (Quest :type "Quest Object Reference"))
  (`self.Reward`))