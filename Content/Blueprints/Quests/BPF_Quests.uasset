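; Blueprint function library of quest helpers for reading and changing quest state by quest ID from anywhere in the game.
; GetQuest takes the first USPlayerController found in the world and returns the valid quest from its QuestComponent.
; The other functions build on that lookup to read or set the current step, or to start or complete the quest.
; Setting a step calls Update only when the value changes, and callers of GetQuest skip validity checks.
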(fn `GetQuest`
  (params (QuestId :type "EQuestList Enum" :default "CooksAssistant"))
  (returns (Quest :type "Quest Object Reference"))
  (bind _outactors (`GameplayStatics.GetAllActorsOfClass` (`local.__WorldContext`) "/Script/UnrealScape.USPlayerController"))
  (if (> (`KismetArrayLibrary.Array_Length` _outactors) 0)
    (bind _returnvalue (`QuestComponent.GetQuest` (`USPlayerController.QuestComponent` (`|GetArrayItem` _outactors)) (`local.QuestId`)))
    (`/Engine/EditorBlueprintResources/StandardMacros.IsValid` _returnvalue
      (:`Is Valid`
        (return _returnvalue)))))

(fn `GetQuestStep`
  (params (QuestId :type "EQuestList Enum" :default "CooksAssistant"))
  (returns (Step :type Integer))
  (return (`Quest.CurrentStep` (`self.GetQuest` QuestId (`local.__WorldContext`)))))

(fn `SetQuestCompleted`
  (params (QuestId :type "EQuestList Enum" :default "CooksAssistant"))
  (`Quest.Complete` (`self.GetQuest` QuestId (`local.__WorldContext`))))

(fn `SetQuestStarted`
  (params (QuestId :type "EQuestList Enum" :default "CooksAssistant"))
  (`Quest.Start` (`self.GetQuest` QuestId (`local.__WorldContext`))))

(fn `SetQuestStep`
  (params (QuestId :type "EQuestList Enum" :default "CooksAssistant") (Step :type Integer))
  (bind _quest (`self.GetQuest` QuestId (`local.__WorldContext`)))
  (if (!= Step (`Quest.CurrentStep` _quest))
    (bind _output_get (set `Quest.CurrentStep` Step _quest))
    (`Quest.Update` _quest _output_get)))