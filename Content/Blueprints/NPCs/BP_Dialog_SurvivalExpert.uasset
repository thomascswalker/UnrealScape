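; Dialogue Blueprint for Brynna, the Tutorial Island survival expert who introduces Fishing, Cooking, Woodcutting and Firemaking.
; The Communicate event is a step-indexed state machine whose opening line depends on the current TutorialIsland quest step.
; NPC and player lines chain through GoToStep, and terminal steps advance the quest and end the dialogue.
; A final quest-completion step exists, but no line here leads to it.
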(event `self.Communicate`
  (params (Step :type Integer))
  (switch `int` Step
    (:`0`
      (switch `int` (`QuestFunctionLibrary.GetQuestStep` null "TutorialIsland")
        (:`2`
          (`DialogAsset.AddNpc` "Hello there, newcomer. My name is Brynna. My job is to teach you about the skills you can use to survive in this world." 1))
        (:`3`
          (`DialogAsset.AddNpc` "Hello again. First up, we're going to do some fishing. There's some shrimp in this pond here. Let's try and catch some." 3))
        (:`4`
          (`DialogAsset.AddPlayer` "I've managed to catch some shrimp." 3))))
    (:`1`
      (`DialogAsset.AddNpc` "The first skill we're going to look at is Fishing. There's some shrimp in this pond here. Let's try and catch some." 2))
    (:`2`
      (`QuestFunctionLibrary.SetQuestStep` null "TutorialIsland" 3)
      (`DialogAsset.EndDialog`))
    (:`3`
      (`DialogAsset.AddNpc` "Excellent work. Now that you have some shrimp, you're going to want to cook them. To do that, you'll need a fire. This brings us on to the Woodcutting and Firemaking skills." 4))
    (:`4`
      (`QuestFunctionLibrary.SetQuestStep` null "TutorialIsland" 5)
      (`DialogAsset.EndDialog`))
    (:`5`
      (`QuestFunctionLibrary.CompleteQuest` null "TutorialIsland")
      (`DialogAsset.EndDialog`))))