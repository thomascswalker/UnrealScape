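; BP_PawnEntity is a data-driven interactive NPC that offers Talk and Examine options.
; Its construction script reads the NPC data table row to set the mesh, dialog asset and interactive component's name, type, options and distance.
; Talk starts that dialog and Examine logs a fixed Gielinor guide description, each then completing the interaction.
; Cursor hover toggles custom depth rendering on the mesh for highlighting.
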(event `self.ReceiveActorBeginCursorOver`
  (`PrimitiveComponent.SetRenderCustomDepth` (`self.SkeletalMeshComponent`) true))

(event `self.ReceiveActorEndCursorOver`
  (`PrimitiveComponent.SetRenderCustomDepth` (`self.SkeletalMeshComponent`) false))

(event `self.Interact`
  (params (Option :type "InteractOption Structure (by ref)"))
  (switch `string` (`.Name` (break `InteractOption` Option))
    (:`Talk`
      (`/Game/Blueprints/UI/FBP_Chatbox.Start Dialog` (`DialogComponent.DialogAssetClass` (`self.DialogComponent`)))
      (`InteractiveComponent.Complete` (`self.InteractiveComponent`)))
    (:`Examine`
      (`/Game/Blueprints/UI/FBP_Chatbox.Log` "Your guide to the world of Gielinor.")
      (`InteractiveComponent.Complete` (`self.InteractiveComponent`)))))

(fn `GetName`
  (returns (ReturnValue :type String))
  (return (`InteractiveComponent.Name` (`self.InteractiveComponent`))))

(fn `UserConstructionScript`
  (bind (_npc_datatable _npc_rowname) (break `DataTableRowHandle` (`self.NPC`)))
  (bind _interactivecomponent (`self.InteractiveComponent`))
  (bind _returnvalue (`|GetDataTableRow` _npc_datatable _npc_rowname)
    (:`then`
      (bind (_dialogasset _skeletalmesh _interactdistance _name _type _options) (break `PawnEntityData` _returnvalue))
      (set `DialogComponent.DialogAssetClass` _dialogasset (`self.DialogComponent`))
      (`SkeletalMeshComponent.SetSkeletalMeshAsset` (`self.SkeletalMeshComponent`) _skeletalmesh)
      (set `InteractiveComponent.InteractDistance` _interactdistance _interactivecomponent)
      (set `InteractiveComponent.Name` _name _interactivecomponent)
      (set `InteractiveComponent.Type` _type _interactivecomponent)
      (set `InteractiveComponent.Options` _options _interactivecomponent))))