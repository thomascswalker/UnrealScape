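; BP_DialogAsset is a dialog asset Blueprint that gives NPC dialog access to the player and the NPC.
; GetPlayer casts the asset's outer object to a DialogInterpreterComponent and returns its owner as a BP_USPlayerController, so it relies on the asset being outered to that component.
; GetNpc returns that controller's TargetEntity as a BP_PawnEntity when the player is valid.
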(fn `GetNpc`
  (returns (Npc :type "/Game/Blueprints/NPCs/BP_PawnEntity Object Reference"))
  (bind _player (`self.GetPlayer`))
  (`/Engine/EditorBlueprintResources/StandardMacros.IsValid` _player
    (:`Is Valid`
      (bind _asbp_pawn_entity (cast `/Game/Blueprints/NPCs/BP_PawnEntity` (`USPlayerController.TargetEntity` _player)))
      (return _asbp_pawn_entity))))

(fn `GetPlayer`
  (returns (Player :type "/Game/Blueprints/BP_USPlayerController Object Reference"))
  (bind _asdialog_interpreter_component (cast `DialogInterpreterComponent` (`KismetSystemLibrary.GetOuterObject` self)))
  (bind _asbp_usplayer_controller (cast `/Game/Blueprints/BP_USPlayerController` (`ActorComponent.GetOwner` _asdialog_interpreter_component)))
  (return _asbp_usplayer_controller))