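; Dialog Blueprint for the Gielinor Guide NPC, which welcomes new arrivals and starts the Tutorial Island quest.
; The Communicate event switches on a step index, queuing NPC lines that each point to the next step.
; The first step starts the quest at stage one if unstarted, otherwise jumps to the last line.
; Only the greeting has text set, and the final step closes the dialog and sets quest stage one again.
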(event `self.Communicate`
  (params (Step :type Integer))
  (bind _returnvalue (`self.GetWorld`))
  (switch `int` Step
    (:`0`
      ;[1 1 1] If we can start this quest
      (if (== (`/Game/Blueprints/Quests/BPF_Quests.GetQuestStep` "TutorialIsland" (`self.GetWorld`)) 0)
        ;[1 1 1] Start the quest
        (`/Game/Blueprints/Quests/BPF_Quests.SetQuestStarted` "TutorialIsland" _returnvalue)
        (`/Game/Blueprints/Quests/BPF_Quests.SetQuestStep` "TutorialIsland" 1 _returnvalue)
        (`self.AddNpc` "Greetings! I see you are a new arrival to the world of Gielinor. My job is to welcome all new visitors. So welcome!" 1)
        (else
          ;[1 1 1] If we've already started, go to the last dialog option
          (`self.Communicate` 3))))
    (:`1`
      (`self.AddNpc` "" 2))
    (:`2`
      (`self.AddNpc` "" 3))
    (:`3`
      (`self.AddNpc` "" 4))
    (:`4`
      (`self.EndDialog`)
      (`/Game/Blueprints/Quests/BPF_Quests.SetQuestStep` "TutorialIsland" 1 (`self.GetWorld`)))))