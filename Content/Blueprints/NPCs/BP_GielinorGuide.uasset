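; Gielinor Guide NPC that welcomes new players and sends them to the tutorial's first instructor.
; Interact switches on the option: Talk builds a staged dialog on DialogComponent, with a continue-or-repeat choice, and starts it through the player controller's DialogInterpreterComponent.
; Examine logs a short description to the chatbox.
; Both options then signal interaction complete, with Talk doing so right after starting the dialog.
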(event `self.Interact`
  (params (Option :type "Option Structure (by ref)"))
  (bind _dialog (`DialogComponent.Dialog` (`self.DialogComponent`)))
  (switch `string` Option_Name
    (:`Talk`
      ;[1 1 1] Dialog
      (`DialogAsset.AddNpcDialog` _dialog " Greetings! I see you are a new arrival to the world of Gielinor. My job is to welcome all new visitors. So welcome!" 0)
      (`DialogAsset.AddNpcDialog` _dialog "You have already learned the first thing needed to succeed in this world: talking to other people!" 5)
      (`DialogAsset.AddNpcDialog` _dialog "You will find many inhabitants of this world have useful things to say to you. By clicking on them you can talk to them." 10)
      (`DialogAsset.AddTwoOptions` _dialog "Do you want me to repeat this?" 15 (make `DialogOption` "No, continue." 20) (make `DialogOption` "Yes, repeat"))
      (`DialogAsset.AddNpcDialog` _dialog "To continue the tutorial go through that door over there and speak to your first instructor!" 20)
      (`DialogAsset.AddEnd` _dialog 25)
      (bind _asbp_usplayer_controller (cast `/Game/Blueprints/BP_USPlayerController` (`GameplayStatics.GetPlayerController` 0)))
      (`DialogInterpreterComponent.Start` (`USPlayerController.DialogInterpreterComponent` _asbp_usplayer_controller) (`DialogComponent.Dialog` (`self.DialogComponent`))))
    (:`Examine`
      (`/Game/Blueprints/UI/FBP_Chatbox.Log (Chatbox)` "Your introduction to the world of Gielinor.")))
  (`GameEntity.InteractionComplete` self))

(fn `UserConstructionScript`)