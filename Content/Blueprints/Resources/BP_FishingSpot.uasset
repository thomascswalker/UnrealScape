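; BP_FishingSpot is a gatherable resource actor where the player catches raw shrimp with a small fishing net.
; Interact checks for the net before calling StartGather, or posts a chat message if it is missing.
; OnGather grants one shrimp with a chat message and ends gathering if the give fails, as does Interrupt.
; Cursor hover toggles custom depth on the mesh.
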(event `self.ReceiveActorBeginCursorOver`
  (`PrimitiveComponent.SetRenderCustomDepth` (`self.StaticMeshComponent`) true))

(event `self.ReceiveActorEndCursorOver`
  (`PrimitiveComponent.SetRenderCustomDepth` (`self.StaticMeshComponent`) false))

(event `self.OnGather`
  (`ItemFunctionLibrary.GivePlayerItemFromId` 317 ; Give the player raw shrimp
    (:`True`
      (`GlobalFunctionLibrary.AddChatboxMessage` "You catch some shrimps."))
    (:`False`
      (`self.EndGather`))))

(event `self.Interact`
  (params (Option :type "InteractOption Structure (by ref)"))
  (switch `string` (`.Name` (break `InteractOption` Option))
    (:`Small net`
      (`ItemFunctionLibrary.PlayerHasItemById` 303 ; Small fishing net
        (:`True`
          (`self.StartGather`))
        (:`False`
          (`GlobalFunctionLibrary.AddChatboxMessage` "You need a small fishing net to fish here."))))))

(event `self.Interrupt`
  (`self.EndGather`))

(fn `UserConstructionScript`)