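; BP_USPlayerController is a player controller that handles camera rotation and click-to-move tile navigation for the USCharacter pawn.
; Holding A or D sets a rotation speed and runs a looping timer that yaws the character's spring arm until release.
; Releasing left click traces under the cursor, refreshes the character's navigator grid and tile, then navigates to the tile at the hit location.
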(event `Key|D`
  (params (Key :type "Key Structure"))
  (:`Pressed`
    (set `self.RotationSpeed` -5.0)
    (bind _returnvalue (`KismetSystemLibrary.K2_SetTimerDelegate` (delegate `CustomEvent`) 0.1 true))
    (set `self.NewVar` _returnvalue))
  (:`Released`
    (set `self.RotationSpeed` 0.0)
    (`KismetSystemLibrary.K2_InvalidateTimerHandle` (`self.NewVar`))))

(event `Key|A`
  (params (Key :type "Key Structure"))
  (:`Pressed`
    (set `self.RotationSpeed` 5.0)
    (bind _returnvalue (`KismetSystemLibrary.K2_SetTimerDelegate` (delegate `CustomEvent`) 0.1 true))
    (set `self.NewVar_0` _returnvalue))
  (:`Released`
    (set `self.RotationSpeed` 0.0)
    (`KismetSystemLibrary.K2_InvalidateTimerHandle` (`self.NewVar_0`))))

(event `CustomEvent`
  (bind _asuscharacter (cast `USCharacter` (`GameplayStatics.GetPlayerPawn` 0)))
  (`SceneComponent.K2_AddRelativeRotation` (`USCharacter.SpringArmComponent` _asuscharacter) (`KismetMathLibrary.MakeRotator` 0.0 0.0 (`self.RotationSpeed`)) true false))

(event `InputAction|LeftClick`
  (params (Key :type "Key Structure"))
  (:`Released`
    (`KismetSystemLibrary.FlushPersistentDebugLines`)
    (bind (_hitresult _returnvalue) (`self.LineTraceUnderMouseCursor`))
    (if _returnvalue
      (bind _asuscharacter (cast `USCharacter` (`GameplayStatics.GetPlayerPawn` 0)))
      (bind _navigatorcomponent (`USCharacter.NavigatorComponent` _asuscharacter))
      (`NavigatorComponent.UpdateCurrentGrid` _navigatorcomponent)
      (`NavigatorComponent.UpdateCurrentTile` _navigatorcomponent)
      (bind _returnvalue_2 (`Grid.GetTileInfoFromLocation` (`NavigatorComponent.CurrentGrid` _navigatorcomponent) (`.Location` (`GameplayStatics.BreakHitResult` _hitresult))))
      (`NavigatorComponent.Navigate` _navigatorcomponent (0.0 0.0 0.0) _returnvalue_2))))

(fn `UserConstructionScript`)