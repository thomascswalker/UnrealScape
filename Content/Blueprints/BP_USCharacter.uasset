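; BP_USCharacter is a character Blueprint holding spring-arm camera rotation and zoom logic, none of which is wired to run.
; Left and right rotation chains set a signed speed and start a looping timer meant to yaw the spring arm, with matching chains that stop it.
; A zoom chain clamps the arm length, but its input is a constant zero.
; No event triggers these chains, and the construction script is empty.
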(fn `UserConstructionScript`)