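; Blueprint function library giving global access to the player's inventory by item Id.
; It finds the InventoryComponent on player 0's BP_USPlayerController and forwards has-item checks and item additions to it.
; Adding first resolves the Id by linearly scanning DT_Items rows for a matching Id field, rather than looking up by row name.
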(fn `Add Item (Id)`
  (params (Id :type Integer))
  (returns (ItemAdded :type Boolean))
  (bind ___worldcontext (`local.__WorldContext`))
  (bind _item (`self.Get Item From Id` Id ___worldcontext))
  (bind _returnvalue (`InventoryComponent.AddItem` (`self.Get Inventory Component` ___worldcontext) _item))
  (return _returnvalue))

(fn `Get Inventory Component`
  (returns (Component :type "InventoryComponent Object Reference"))
  (bind _asbp_usplayer_controller (cast `/Game/Blueprints/BP_USPlayerController` (`GameplayStatics.GetPlayerController` (`local.__WorldContext`))))
  (return (`USPlayerController.InventoryComponent` _asbp_usplayer_controller)))

(fn `Get Item From Id`
  (params (Id :type Integer))
  (returns (Item :type "Item Structure"))
  (bind _outrownames (`DataTableFunctionLibrary.GetDataTableRowNames` "/Game/Blueprints/Items/DT_Items.DT_Items"))
  (for _array_element _outrownames
    (bind _returnvalue (`|GetDataTableRow` "/Game/Blueprints/Items/DT_Items.DT_Items" _array_element)
      (:`then`
        (if (== (`.Id` (break `Item` _returnvalue)) (`local.Id`))
          (return _returnvalue))))))

(fn `Has Item (Id)`
  (params (Id :type Integer))
  (returns (HasItem :type Boolean))
  (`InventoryComponent.HasItemId` (`self.Get Inventory Component` (`local.__WorldContext`)) Id
    (:`True`
      (return true))
    (:`False`
      (return false))))