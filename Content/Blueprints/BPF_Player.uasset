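; BPF_Player is a function library that exposes the player's hint system as global calls for creating and clearing hints.
; CreateHint passes a location and a clear-hints flag to the HintComponent on the first player controller, and ClearHints forwards a clear request to it.
; Both functions cast that controller to USPlayerController and do nothing if the cast fails.
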(fn `ClearHints`
  (bind _asusplayer_controller (cast `USPlayerController` (`GameplayStatics.GetPlayerController` (`local.__WorldContext`))))
  (`HintComponent.ClearHints` (`USPlayerController.HintComponent` _asusplayer_controller)))

(fn `CreateHint`
  (params (Location :type "Vector Structure") (ClearHints :type Boolean))
  (bind _asusplayer_controller (cast `USPlayerController` (`GameplayStatics.GetPlayerController` (`local.__WorldContext`))))
  (`HintComponent.CreateHint` (`USPlayerController.HintComponent` _asusplayer_controller) (`local.Location`) (`local.ClearHints`)))